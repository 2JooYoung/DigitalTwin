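; BP_AMR is an early-stage AMR actor that simulates a draining battery.
; A looping timer set on BeginPlay lowers Battery at a fixed rate with no lower limit.
; Tick prints the battery level in red as debug output, along with a doubled delta time.
; AI movement toward a BP_Rack and a clamp node are present but unconnected, so the Blueprint never issues movement.
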(event `self.ReceiveTick`
  (params (DeltaSeconds :type "Float (single-precision)"))
  (bind _output_get (set `self.Delta Seconds` (+ DeltaSeconds (`self.Delta Seconds`))))
  (`KismetSystemLibrary.PrintString` (`KismetStringLibrary.Conv_DoubleToString` _output_get) true true (struct :`G` 0.66 :`B` 1.0 :`A` 1.0) 0.0)
  (`KismetSystemLibrary.PrintString` (`KismetStringLibrary.Conv_DoubleToString` (`self.Battery`)) true true (struct :`R` 1.0 :`G` 0.043884 :`B` 0.041497 :`A` 1.0) 0.0))

(event `self.ReceiveBeginPlay`
  (`KismetSystemLibrary.K2_SetTimerDelegate` (delegate `Decrease Battery`) 2.0 true))

(event `Decrease Battery`
  (set `self.Battery` (- (`self.Battery`) 1.0)))

(fn `UserConstructionScript`)